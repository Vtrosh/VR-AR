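; Blueprint actor that moves its MovingObject component back and forth along a direction picked from DirectionArray.
; Each Tick applies a swept relative offset scaled by Speed and delta time, with StepNumberI modulo 3 selecting the direction.
; The ObjectMove flag reverses travel when the largest relative coordinate reaches 500 or the smallest drops to -1.
; PlatformIsPressed exposes a StepNumberI parameter but has no logic of its own.
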(event EventTick
  (params (DeltaSeconds :type Float%20%28single-precision%29))
  (bind _movingobject (Variables|Default|GetMovingObject))
  (bind _relativelocation (Variables|/Script/Engine.SceneComponent|GetRelativeLocation _movingobject))
  (if (Variables|Default|GetObjectMove)
    (Transformation|AddRelativeLocation (Variables|Default|GetMovingObject) (* (* (Utilities|Array|Get(acopy) (Variables|Default|GetDirection_Array) (Math|Integer|%(Integer) (stale EventPlatformIsPressed StepNumberI) 3)) (Variables|Default|GetSpeed)) DeltaSeconds) true false)
    (if (not (< (Math|Float|Max(Float) (.x _relativelocation) (.y _relativelocation) (.z _relativelocation)) 5e+02))
      (Variables|Default|SetObjectMove false))
    (else
      (Transformation|AddRelativeLocation (Variables|Default|GetMovingObject) (* (* (* (Utilities|Array|Get(acopy) (Variables|Default|GetDirection_Array) (Math|Integer|%(Integer) (stale EventPlatformIsPressed StepNumberI) 3)) (Variables|Default|GetSpeed)) DeltaSeconds) -1) true false)
      (if (not (> (Math|Float|Min(Float) (.x _relativelocation) (.y _relativelocation) (.z _relativelocation)) -1.0))
        (Variables|Default|SetObjectMove true)))))

(event EventPlatformIsPressed
  (params (StepNumberI :type Integer)))

(fn ConstructionScript)