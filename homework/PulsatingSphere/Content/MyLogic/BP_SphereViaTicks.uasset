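; BP_SphereViaTicks is a Blueprint that pulses a Sphere component between normal and double scale, driven by Tick.
; Each frame it lerps the relative scale from CurrentScale toward TargetScale using DeltaSeconds times ScaleSpeed, then stores the world scale as CurrentScale.
; When CurrentScale nears the target within a small tolerance, it flips Growing and swaps the target, with Growing true selecting the smaller size.
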(event EventTick
  (params (DeltaSeconds :type Float%20%28single-precision%29))
  (Transformation|SetRelativeScale3D (Variables|Default|GetSphere) (Math|Vector|Lerp(Vector) (Variables|Default|GetCurrentScale) (Variables|Default|GetTargetScale) (* DeltaSeconds (Variables|Default|GetScaleSpeed))))
  (bind _output_get (Variables|Default|SetCurrentScale (Transformation|GetWorldScale (Variables|Default|GetSphere))))
  (if (Math|Vector|Equal(Vector) _output_get (Variables|Default|GetTargetScale) 0.03)
    (bind _output_get_2 (Variables|Default|SetGrowing (not (Variables|Default|GetGrowing))))
    (if _output_get_2
      (Variables|Default|SetTargetScale "1.000000,1.000000,1.000000")
      (else
        (Variables|Default|SetTargetScale "2.000000,2.000000,2.000000")))))

(fn ConstructionScript)