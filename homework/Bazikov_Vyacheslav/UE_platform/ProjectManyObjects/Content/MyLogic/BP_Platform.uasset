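; BP_Platform is a pressure platform that counts how many times a ThirdPersonCharacter steps onto it.
; Each begin overlap on its Box by that character increments StepNumber and sends it through PlatformIsPressedMessage to all actors implementing BP_Interface, so listeners need no direct reference.
; Tick prints the running count on screen in Russian every frame, using the frame delta as the display duration.
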(event OnComponentBeginOverlap(Box)
  (params (OverlappedComponent :type Primitive%20Component%20Object%20Reference) (OtherActor :type Actor%20Object%20Reference) (OtherComp :type Primitive%20Component%20Object%20Reference) (OtherBodyIndex :type Integer) (bFromSweep :type Boolean) (SweepResult :type Hit%20Result%20Structure%20%28by%20ref%29))
  (Utilities|Casting|CastToThirdPersonCharacter OtherActor)
  (Variables|Default|SetStepNumber (+ (Variables|Default|GetStepNumber) 1))
  (bind _outactors (Actor|GetAllActorswithInterface "/Game/MyLogic/BP_Interface.BP_Interface_C"))
  (Class|BPInterface|PlatformIsPressed(Message) _outactors (Variables|Default|GetStepNumber)))

(event EventTick
  (params (DeltaSeconds :type Float%20%28single-precision%29))
  (Development|PrintString (Utilities|String|Append "Наступили на платформу " (Utilities|String|ToString(Integer) (Variables|Default|GetStepNumber)) " раз.") true true "(R=0.000000,G=0.660000,B=1.000000,A=1.000000)" DeltaSeconds))

(fn ConstructionScript)